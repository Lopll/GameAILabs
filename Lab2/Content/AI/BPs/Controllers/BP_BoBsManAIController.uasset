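; AI controller that makes its pawn wander between random navmesh points around its current location.
; BeginPlay picks a random navigable point within a fixed radius, and Tick issues AIMoveTo toward it, choosing a new reachable point on each success.
; Unconnected alternatives remain in the graph for moving to TargetPoint actors, stepping through them in sequence, or following the player.
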(event EventBeginPlay
  (bind _randomlocation (Class|NavigationSystemV1|GetRandomLocationinNavigableRadius (Transformation|GetActorLocation (Pawn|GetControlledPawn)) 1e+03 0 0))
  (Variables|Default|SetRndTargetPoint _randomlocation))

(event EventTick
  (params (DeltaSeconds :type Float%20%28single-precision%29))
  (AI|AIMoveTo 0 (Variables|Default|GetRndTargetPoint) 0 5.0 false
    (:OnSuccess
      (Variables|Default|SetRndTargetPoint (.RandomLocation (AI|Navigation|GetRandomReachablePointinRadius (Transformation|GetActorLocation (Pawn|GetControlledPawn)) 1e+03 0 0))))))

(fn ConstructionScript)