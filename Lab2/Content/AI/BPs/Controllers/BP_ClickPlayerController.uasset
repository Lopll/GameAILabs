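; BP_ClickPlayerController is a click-to-move player controller that shows the mouse cursor.
; A left click stores the complex Visibility trace hit under the cursor as Goal, which starts at the pawn's location.
; Tick steers player pawn 0 straight toward Goal with movement input, without pathfinding or an arrival check.
; It also forwards Jump input to the character and caches a BP_Player reference, unused here.
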(event EventBeginPlay
  (bind _returnvalue (Game|Player|GetPlayerPawn 0))
  ;[1 1 1] BeginPlay
  (Variables|Default|SetbShowMouseCursor true)
  (bind _asbp_player (Utilities|Casting|CastToBP_Player _returnvalue))
  (Variables|Default|SetPlayerRef _asbp_player)
  (Variables|Default|SetGoal (Transformation|GetActorLocation _returnvalue)))

(event EventTick
  (params (DeltaSeconds :type Float%20%28single-precision%29))
  (bind _returnvalue (Game|Player|GetPlayerPawn 0))
  ;[1 1 1] Tick
  (Pawn|Input|AddMovementInput _returnvalue (Math|Vector|GetUnitDirection(Vector) (Transformation|GetActorLocation _returnvalue) (Variables|Default|GetGoal)) 2e+01 false))

(event Input|ActionEvents|InputActionJump
  (params (Key :type Key%20Structure :default "None"))
  (bind _returnvalue (Game|GetPlayerCharacter 0))
  ;[1 1 1] Jump (взятый из стандартного персонажа)
  (:Pressed
    (Character|Jump _returnvalue))
  (:Released
    (Character|StopJumping _returnvalue)))

(event Input|MouseEvents|LeftMouseButton
  (params (Key :type Key%20Structure :default "None"))
  ;[1 1 1] LeftMouseButtonInput
  (:Pressed
    (Variables|Default|SetGoal (.Location (Collision|BreakHitResult (.HitResult (Game|Player|GetHitResultUnderCursorbyChannel "TraceTypeQuery1" true)))))))

(fn ConstructionScript)