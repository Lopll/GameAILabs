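; BP_SimpleAIController is a basic wandering AI controller that keeps its pawn moving and turns it when something blocks the view ahead.
; Each Tick it runs a debug-drawn Visibility line trace along the pawn's forward vector.
; On a hit it yaws the stored Direction by a small step, choosing left or right at random each frame.
; It then feeds Direction into AddMovementInput, without navigation or behavior trees.
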(event EventBeginPlay)

(event EventTick
  (params (DeltaSeconds :type Float%20%28single-precision%29))
  (bind _returnvalue (Pawn|GetControlledPawn))
  (bind _returnvalue_2 (Transformation|GetActorLocation _returnvalue))
  (bind _returnvalue_3 (Collision|LineTraceByChannel _returnvalue_2 (+ _returnvalue_2 (* (Transformation|GetActorForwardVector _returnvalue) 500)) "TraceTypeQuery1" false 0 "ForOneFrame"))
  (if _returnvalue_3
    (Variables|Default|SetRandDirection (select (Math|Random|RandomBool) -5.0 5.0))
    (Variables|Default|SetDirection (Math|Vector|RotateVector (Variables|Default|GetDirection) (Math|Rotator|MakeRotator 0.0 0.0 (Variables|Default|GetRandDirection)))))
  (Pawn|Input|AddMovementInput (Pawn|GetControlledPawn) (Variables|Default|GetDirection) 1.0 false))

(fn ConstructionScript)