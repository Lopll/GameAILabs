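; BP_BoBon is a self-steering pawn that moves constantly and turns away from obstacles using visibility line traces.
; Each Tick, a forward trace hit triggers a right trace, turning right 15 degrees if clear or left 45 degrees if blocked.
; The left trace's result is unused, leaving the gentler left turn unreachable.
; MoveWithRotation rotates a stored Direction for movement input, while ToggleWasRotated blocks further turns for 0.2 seconds.
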(event EventBeginPlay)

(event Collision|EventActorBeginOverlap
  (params (OtherActor :type Actor%20Object%20Reference)))

(event EventTick
  (params (DeltaSeconds :type Float%20%28single-precision%29))
  (bind _returnvalue (Transformation|GetActorLocation))
  (bind _returnvalue_2 (Transformation|GetActorLocation))
  (bind _returnvalue_3 (Transformation|GetActorLocation))
  ;[1 1 1] PlaceForwardTrace
  (bind _returnvalue_4 (Collision|LineTraceByChannel _returnvalue_2 (+ _returnvalue_2 (* (Transformation|GetActorForwardVector) (Variables|Default|GetRayLen))) "TraceTypeQuery1" false 0 "ForOneFrame"))
  (if (and _returnvalue_4 (not (Variables|Default|GetWasRotated)))
    ;[1 1 1] PlaceRightTrace
    (bind _returnvalue_5 (Collision|LineTraceByChannel _returnvalue_3 (+ _returnvalue_3 (* (Transformation|GetActorRightVector) (Variables|Default|GetRayLen))) "TraceTypeQuery1" false 0 "ForOneFrame"))
    (if _returnvalue_5
      ;[1 1 1] PlaceRightTrace
      (Collision|LineTraceByChannel _returnvalue (+ _returnvalue (* (Transformation|GetActorRightVector) (* (Variables|Default|GetRayLen) -1))) "TraceTypeQuery1" false 0 "ForOneFrame")
      (if true
        (Variables|Default|SetRotation "0,-45.000000, 0") ; Move gigaleft
        (Utilities|MovewithRotation)
        (Utilities|ToggleWasRotated)
        (else
          (Variables|Default|SetRotation "0,-15.000000, 0") ; Move left
          (Utilities|MovewithRotation)
          (Utilities|ToggleWasRotated)))
      (else
        (Variables|Default|SetRotation "0,15.000000, 0") ; Move right
        (Utilities|MovewithRotation)
        (Utilities|ToggleWasRotated)))
    (else
      (Variables|Default|SetRotation "0, 0, 0") ; Move forward
      (Utilities|MovewithRotation))))

(fn ConstructionScript)